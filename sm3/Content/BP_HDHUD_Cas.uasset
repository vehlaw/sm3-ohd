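; HUD Blueprint that draws a dynamic four-point crosshair at screen centre.
; Each DrawHUD pass hands a self reference to the owning player's BP_HDPlayerCharacter_Cas, then draws a fixed centre texture and four arms.
; The arms reuse one texture rotated per side, shifted by CrosshairOffset and CrosshairDefaultSpread and faded by CrosshairAlpha, none of which are set in this Blueprint.
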(event EventDrawHUD
  (params (SizeX :type Integer) (SizeY :type Integer))
  (bind _returnvalue (/ SizeY 2))
  (bind _returnvalue_2 (/ SizeX 2))
  (bind _crosshair_offset (Variables|Default|GetCrosshair%20Offset))
  (bind _crosshair_alpha (Variables|Default|GetCrosshair%20Alpha))
  (bind _crosshair_default_spread (Variables|Default|GetCrosshair%20Default%20Spread))
  (bind _returnvalue_3 (Math|Conversions|ToFloat(Integer) _crosshair_offset))
  (bind _returnvalue_4 (- _returnvalue 8))
  (bind _returnvalue_5 (Math|Conversions|ToFloat(Integer) _crosshair_default_spread))
  (bind _returnvalue_6 (- _returnvalue_2 8))
  (bind _linearcolor (Utilities|Struct|MakeLinearColor 1.0 1.0 1.0 _crosshair_alpha))
  (bind _returnvalue_7 (/ _returnvalue_3 6.0))
  (bind _returnvalue_8 (- 96.0 _returnvalue_5))
  (bind _returnvalue_9 (Math|Conversions|ToFloat(Integer) _returnvalue_4))
  (bind _returnvalue_10 (Math|Conversions|ToFloat(Integer) _returnvalue_6))
  (bind _returnvalue_11 (* _returnvalue_7 -1.0))
  (bind _returnvalue_12 (+ _returnvalue_11 _returnvalue_8))
  (bind _output_get (Variables|Default|SetHUD self))
  (Variables|/CasualMod/BP_HDPlayerCharacter_Cas.BP_HDPlayerCharacter_Cas_C|SetHUD (.AsBP%20HDPlayer%20Character%20Cas (Utilities|Casting|CastToBP_HDPlayerCharacter_Cas (CallFunction|GetHDPlayerCharacterBP (Class|GameplayStatics|GetPlayerControllerID (Game|Player|GetOwningPlayerController))))) _output_get)
  (Canvas|DrawTexture "/CasualMod/img/FourPointXHairCenter.FourPointXHairCenter" (- _returnvalue_10 96.0) (- _returnvalue_9 96.0) 192.0 192.0 0.0 0.0 1.0 1.0 "(R=1.000000,G=1.000000,B=1.000000,A=1.000000)")
  (Canvas|DrawTexture "/CasualMod/img/FourPointXHair.FourPointXHair" (- _returnvalue_10 96.0) (- _returnvalue_9 _returnvalue_12) 192.0 192.0 0.0 0.0 1.0 1.0 _linearcolor)
  (Canvas|DrawTexture "/CasualMod/img/FourPointXHair.FourPointXHair" (+ _returnvalue_10 _returnvalue_12) (- _returnvalue_9 96.0) 192.0 192.0 0.0 0.0 1.0 1.0 _linearcolor "BLEND_Translucent" 1.0 false 9e+01)
  (Canvas|DrawTexture "/CasualMod/img/FourPointXHair.FourPointXHair" (- _returnvalue_10 _returnvalue_12) (+ _returnvalue_9 96.0) 192.0 192.0 0.0 0.0 1.0 1.0 _linearcolor "BLEND_Translucent" 1.0 false -9e+01)
  (Canvas|DrawTexture "/CasualMod/img/FourPointXHair.FourPointXHair" (+ _returnvalue_10 96.0) (+ _returnvalue_9 _returnvalue_12) 192.0 192.0 0.0 0.0 1.0 1.0 _linearcolor "BLEND_Translucent" 1.0 false 1.8e+02))

(fn ConstructionScript
  (|CallParentFunction))