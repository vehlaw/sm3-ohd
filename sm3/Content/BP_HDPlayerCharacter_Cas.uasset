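; Player character Blueprint that adds a dynamic crosshair, a sprint-to-crouch slide and firing while prone.
; Timelines fade the crosshair for sprint and aim, while Tick sets its spread from velocity and stance and hides it during slides.
; Sliding temporarily overrides movement speed, friction and braking, duplicated in SlideEvent with a server-named timeline, and uses crouch speed as its state flag.
; Prone firing disables movement until fire is released.
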(event Custom|initTimeline
  (bind _hud (Variables|Default|GetHUD))
  ;[1 1 1] (Required For Crosshair Only)
  (bind _fade (Timeline|FadeOutXHairAim SetNewTime)
    (:Update
      (Utilities|IsValid _hud
        (:Is%20Valid
          (Variables|/sm3/BP_HDHUD_Cas.BP_HDHUD_Cas_C|SetCrosshair%20Alpha _hud _fade)
          (Variables|/sm3/BP_HDHUD_Cas.BP_HDHUD_Cas_C|SetCrosshair%20Offset (Variables|Default|GetHUD) (Utilities|String|ToString(Float) (* _fade (Math|Vector|VectorLength (Variables|/Script/Engine.MovementComponent|GetVelocity (Variables|Default|GetDFCharacterMovement))))))
          (Variables|/sm3/BP_HDHUD_Cas.BP_HDHUD_Cas_C|SetCrosshair%20Default%20Spread (Variables|Default|GetHUD) (Utilities|String|ToString(Float) (* _fade (Math|Conversions|ToFloat(Integer) (Variables|Default|GetRecDefaultSpread))))))))))

(event Custom|SlideCheck
  (bind _dfcharactermovement (Variables|Default|GetDFCharacterMovement))
  ;[1 1 1] (Required For Crosshair & Slide Together)
  (Variables|Default|SetisSliding false)
  (if (AI|Components|NavMovement|IsCrouching _dfcharactermovement)
    (if (not (== (Variables|/Script/Engine.CharacterMovementComponent|GetMaxWalkSpeedCrouched _dfcharactermovement) 2.2e+02))
      (Variables|Default|SetisSliding true)
      (Variables|/sm3/BP_HDHUD_Cas.BP_HDHUD_Cas_C|SetCrosshair%20Alpha (Variables|Default|GetHUD) 0.0))))

(event Custom|SlideEvent
  (bind _dfcharactermovement (Variables|Default|GetDFCharacterMovement))
  ;[1 1 1] (Required For Slide Only)
  (Variables|/Script/Engine.CharacterMovementComponent|SetMaxWalkSpeedCrouched _dfcharactermovement 1.2e+03)
  (Variables|/Script/Engine.CharacterMovementComponent|SetMaxAcceleration _dfcharactermovement 1.2e+04)
  (Variables|/Script/Engine.CharacterMovementComponent|SetGroundFriction _dfcharactermovement 0.0)
  (Variables|/Script/Engine.CharacterMovementComponent|SetBrakingDecelerationWalking _dfcharactermovement 0.0)
  (Utilities|FlowControl|Delay 0.25)
  (Variables|/Script/Engine.CharacterMovementComponent|SetMaxWalkSpeedCrouched _dfcharactermovement 0.0)
  (Variables|/Script/Engine.CharacterMovementComponent|SetMaxAcceleration _dfcharactermovement 0.0)
  (bind _slidetl (Timeline|SlideTLServer PlayFromStart)
    (:Update
      (Variables|/Script/Engine.CharacterMovementComponent|SetGroundFriction _dfcharactermovement _slidetl))
    (:Finished
      (Variables|/Script/Engine.CharacterMovementComponent|SetMaxWalkSpeedCrouched _dfcharactermovement 2.2e+02)
      (Variables|/Script/Engine.CharacterMovementComponent|SetMaxAcceleration _dfcharactermovement 9e+02)
      (Variables|/Script/Engine.CharacterMovementComponent|SetGroundFriction _dfcharactermovement 3.5)
      (Variables|/Script/Engine.CharacterMovementComponent|SetBrakingDecelerationWalking _dfcharactermovement 1024.0))))

(event EventOnStartCrouch
  (params (HalfHeightAdjust :type Float%20%28single-precision%29) (ScaledHalfHeightAdjust :type Float%20%28single-precision%29))
  (bind _dfcharactermovement (Variables|Default|GetDFCharacterMovement))
  ;[1 1 1] (Required For Slide Only)
  (|CallParentFunction HalfHeightAdjust ScaledHalfHeightAdjust)
  (if (Class|DFCharacterMovementComponent|IsSprinting (Variables|Default|GetDFCharacterMovement))
    (if (== (Variables|/Script/Engine.CharacterMovementComponent|GetMaxWalkSpeedCrouched (Variables|Default|GetDFCharacterMovement)) 2.2e+02)
      (Audio|PlaySound2D "/sm3/audio/SlideA.SlideA" 1.0 1.0 0.0 0 0)
      (CallFunction|SlideEvent)
      (Variables|/Script/Engine.CharacterMovementComponent|SetMaxWalkSpeedCrouched _dfcharactermovement 1.2e+03)
      (Variables|/Script/Engine.CharacterMovementComponent|SetMaxAcceleration _dfcharactermovement 1.2e+04)
      (Variables|/Script/Engine.CharacterMovementComponent|SetGroundFriction _dfcharactermovement 0.0)
      (Variables|/Script/Engine.CharacterMovementComponent|SetBrakingDecelerationWalking _dfcharactermovement 0.0)
      (Utilities|FlowControl|Delay 0.25)
      (Variables|/Script/Engine.CharacterMovementComponent|SetMaxWalkSpeedCrouched _dfcharactermovement 0.0)
      (Variables|/Script/Engine.CharacterMovementComponent|SetMaxAcceleration _dfcharactermovement 0.0)
      (bind _slidetl (Timeline|SlideTL PlayFromStart)
        (:Update
          (Variables|/Script/Engine.CharacterMovementComponent|SetGroundFriction _dfcharactermovement _slidetl))
        (:Finished
          (Variables|/Script/Engine.CharacterMovementComponent|SetMaxWalkSpeedCrouched _dfcharactermovement 2.2e+02)
          (Variables|/Script/Engine.CharacterMovementComponent|SetMaxAcceleration _dfcharactermovement 9e+02)
          (Variables|/Script/Engine.CharacterMovementComponent|SetGroundFriction _dfcharactermovement 3.5)
          (Variables|/Script/Engine.CharacterMovementComponent|SetBrakingDecelerationWalking _dfcharactermovement 1024.0))))))

(event EventOnEndAim
  (bind _hud (Variables|Default|GetHUD))
  ;[1 1 1] (Required For Crosshair Only)
  (Utilities|IsValid (Variables|Default|GetHUD)
    (:Is%20Valid
      (bind _fade (Timeline|FadeOutXHairAim Reverse)
        (:Update
          (Utilities|IsValid _hud
            (:Is%20Valid
              (Variables|/sm3/BP_HDHUD_Cas.BP_HDHUD_Cas_C|SetCrosshair%20Alpha _hud _fade)
              (Variables|/sm3/BP_HDHUD_Cas.BP_HDHUD_Cas_C|SetCrosshair%20Offset (Variables|Default|GetHUD) (Utilities|String|ToString(Float) (* _fade (Math|Vector|VectorLength (Variables|/Script/Engine.MovementComponent|GetVelocity (Variables|Default|GetDFCharacterMovement))))))
              (Variables|/sm3/BP_HDHUD_Cas.BP_HDHUD_Cas_C|SetCrosshair%20Default%20Spread (Variables|Default|GetHUD) (Utilities|String|ToString(Float) (* _fade (Math|Conversions|ToFloat(Integer) (Variables|Default|GetRecDefaultSpread))))))))))))

(event EventOnPCFireReleased
  ;[1 1 1] (Required For Prone Firing Only)
  (Pawn|Components|CharacterMovement|SetMovementMode (Variables|Default|GetDFCharacterMovement) "MOVE_Walking" 0))

(event EventOnPCFirePressed
  (bind _dfcharactermovement (Variables|Default|GetDFCharacterMovement))
  ;[1 1 1] (Required For Prone Firing Only)
  (if (Class|DFCharacterMovementComponent|IsProne _dfcharactermovement)
    (if (Variables|Default|GetcanFireProne)
      (Pawn|Components|CharacterMovement|DisableMovement _dfcharactermovement))))

(event EventBeginPlay
  ;[1 1 1] (Required For Crosshair Only)
  (|CallParentFunction)
  (CallFunction|InitTimeline))

(event EventTick
  (params (DeltaSeconds :type Float%20%28single-precision%29))
  (bind _dfcharactermovement (Variables|Default|GetDFCharacterMovement))
  (bind _hud (Variables|Default|GetHUD))
  ;[1 1 1] (Required For Crosshair Only)
  (|CallParentFunction DeltaSeconds)
  (Utilities|IsValid (Variables|Default|GetHUD)
    (:Is%20Valid
      (if (not (Class|DFCharacterMovementComponent|IsAiming (Variables|Default|GetDFCharacterMovement)))
        (CallFunction|SlideCheck)
        (if (not (Variables|Default|GetisSliding))
          (if (== (stale Custom|initTimeline _fade) 1.0)
            (if (not (Class|DFCharacterMovementComponent|IsSprinting _dfcharactermovement))
              (Variables|/sm3/BP_HDHUD_Cas.BP_HDHUD_Cas_C|SetCrosshair%20Alpha (Variables|Default|GetHUD) 0.0)
              (if (Class|DFBaseItem|CanFire (Variables|Default|GetEquippedWeapon))
                _
                (elif (Class|DFCharacterMovementComponent|IsProne _dfcharactermovement)
                  (if (Variables|Default|GetcanFireProne)
                    (Variables|/sm3/BP_HDHUD_Cas.BP_HDHUD_Cas_C|SetCrosshair%20Alpha _hud 0.0)
                    (else
                      (Variables|/sm3/BP_HDHUD_Cas.BP_HDHUD_Cas_C|SetCrosshair%20Alpha _hud 0.0 :!label _label)))
                  (else
                    (goto _label))))
              (Variables|/sm3/BP_HDHUD_Cas.BP_HDHUD_Cas_C|SetCrosshair%20Offset (Variables|Default|GetHUD) (Utilities|String|ToString(Integer) (Math|Float|Round (Math|Vector|VectorLength (Variables|/Script/Engine.MovementComponent|GetVelocity _dfcharactermovement)))))
              (if (Class|DFCharacterMovementComponent|IsProne (Variables|Default|GetDFCharacterMovement))
                (Variables|/sm3/BP_HDHUD_Cas.BP_HDHUD_Cas_C|SetCrosshair%20Default%20Spread (Variables|Default|GetHUD) "12")
                (elif (AI|Components|NavMovement|IsCrouching (Variables|Default|GetDFCharacterMovement))
                  (Variables|/sm3/BP_HDHUD_Cas.BP_HDHUD_Cas_C|SetCrosshair%20Default%20Spread (Variables|Default|GetHUD) "24")
                  (else
                    (Variables|/sm3/BP_HDHUD_Cas.BP_HDHUD_Cas_C|SetCrosshair%20Default%20Spread (Variables|Default|GetHUD) "36")))))))))))

(event EventOnStartSprint
  ;[1 1 1] (Required For Crosshair Only)
  (Utilities|IsValid (Variables|Default|GetHUD)
    (:Is%20Valid
      (bind _fade (Timeline|FadeOutXHair Play)
        (:Update
          (Variables|/sm3/BP_HDHUD_Cas.BP_HDHUD_Cas_C|SetCrosshair%20Alpha (Variables|Default|GetHUD) _fade))))))

(event EventOnEndSprint
  ;[1 1 1] (Required For Crosshair Only)
  (Utilities|IsValid (Variables|Default|GetHUD)
    (:Is%20Valid
      (bind _fade (Timeline|FadeOutXHair Reverse)
        (:Update
          (Variables|/sm3/BP_HDHUD_Cas.BP_HDHUD_Cas_C|SetCrosshair%20Alpha (Variables|Default|GetHUD) _fade))))))

(event EventOnStartAim
  (bind _hud (Variables|Default|GetHUD))
  (bind _hud_2 (Variables|Default|GetHUD))
  ;[1 1 1] (Required For Crosshair Only)
  (Utilities|IsValid _hud_2
    (:Is%20Valid
      (Variables|Default|SetRecDefaultSpread (Variables|/sm3/BP_HDHUD_Cas.BP_HDHUD_Cas_C|GetCrosshair%20Default%20Spread _hud_2))
      (bind _fade (Timeline|FadeOutXHairAim Play)
        (:Update
          (Utilities|IsValid _hud
            (:Is%20Valid
              (Variables|/sm3/BP_HDHUD_Cas.BP_HDHUD_Cas_C|SetCrosshair%20Alpha _hud _fade)
              (Variables|/sm3/BP_HDHUD_Cas.BP_HDHUD_Cas_C|SetCrosshair%20Offset (Variables|Default|GetHUD) (Utilities|String|ToString(Float) (* _fade (Math|Vector|VectorLength (Variables|/Script/Engine.MovementComponent|GetVelocity (Variables|Default|GetDFCharacterMovement))))))
              (Variables|/sm3/BP_HDHUD_Cas.BP_HDHUD_Cas_C|SetCrosshair%20Default%20Spread (Variables|Default|GetHUD) (Utilities|String|ToString(Float) (* _fade (Math|Conversions|ToFloat(Integer) (Variables|Default|GetRecDefaultSpread))))))))))))

(fn ConstructionScript
  (|CallParentFunction))